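; Player character Blueprint that sets up the tray inventory and HUD when play begins.
; BeginPlay spawns a BP_TrayInventory actor at the player's transform with the requested slot count and a player reference, then shows the mouse cursor.
; It then creates the HUD widget with that inventory reference and adds it to the viewport.
; The inventory receives HUDRef at spawn, before this graph assigns it.
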(event EventBeginPlay
  (bind _self self)
  (bind _returnvalue (Game|SpawnActorfromClass "/Game/Blueprints/BP_TrayInventory.BP_TrayInventory_C" (Transformation|GetActorTransform _self) "AlwaysSpawn" 0 (Variables|Default|GetrequestedAmoutOfTraySlots) _self (Variables|Default|GetHUD_Ref) 0))
  (Variables|Default|SetInventory_Ref _returnvalue)
  (Variables|/Script/Engine.PlayerController|SetbShowMouseCursor (Game|GetPlayerController 0) true)
  (bind _returnvalue_2 (UserInterface|CreateWidget "/Game/UI/WBP_HUD.WBP_HUD_C" (Game|GetPlayerController 0) (Variables|Default|GetInventory_Ref)))
  (bind _output_get (Variables|Default|SetHUD_Ref _returnvalue_2))
  (UserInterface|Viewport|AddtoViewport _output_get 0))

(fn ConstructionScript)