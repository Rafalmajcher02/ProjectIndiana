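; PC_Player is the player controller for a 2D canteen game, handling input setup and pausing.
; On BeginPlay it caches the BP_PlayerCharacter, sets Game and UI input mode, and adds the IMC_Main Enhanced Input mapping context.
; The IA_Pause action toggles pause by calling PauseGameEvent on GMB_2D_CanteenGameMode with the inverse of its IsPaused state.
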(event Input|EnhancedActionEvents|EnhancedInputActionIA_Pause
  (params (ActionValue :type Boolean) (ElapsedSeconds :type Float%20%28double-precision%29) (TriggeredSeconds :type Float%20%28double-precision%29) (InputAction :type Input%20Action%20Object%20Reference :default "/Game/Player/Input/IA_Pause.IA_Pause"))
  (:Started
    (bind _asgmb_2d_canteen_game_mode (Utilities|Casting|CastToGMB_2D_CanteenGameMode (Game|GetGameMode)))
    (Default|PauseGameEvent _asgmb_2d_canteen_game_mode (not (Variables|/Game/Player/GMB_2D_CanteenGameMode.GMB_2D_CanteenGameMode_C|GetisPaused _asgmb_2d_canteen_game_mode)))))

(event EventBeginPlay
  (bind _asbp_player_character (Utilities|Casting|CastToBP_PlayerCharacter (Game|GetPlayerCharacter 0)))
  (Variables|Default|SetplayerRef _asbp_player_character)
  (Input|SetInputModeGameandUI (Game|GetPlayerController 0) 0 "DoNotLock" false false)
  (bind _asplayer_controller (Utilities|Casting|CastToPlayerController (Pawn|GetController (Variables|Default|GetplayerRef))))
  (Utilities|IsValid (PlayerController|LocalPlayerSubsystems|GetEnhancedInputLocalPlayerSubsystem _asplayer_controller)
    (:Is%20Valid
      (Input|AddMappingContext (PlayerController|LocalPlayerSubsystems|GetEnhancedInputLocalPlayerSubsystem _asplayer_controller) "/Game/Player/Input/IMC_Main.IMC_Main" 0 "(bIgnoreAllPressedKeysUntilRelease=True,bForceImmediately=False)"))))

(fn ConstructionScript)