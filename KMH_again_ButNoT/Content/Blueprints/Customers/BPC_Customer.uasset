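; Customer actor for a canteen that builds randomized kid looks and tells the HUD's canteen widget to run KidSprite on BeginPlay.
; GenerateLook rolls a body type to pick matching clothing, blazer and skin tone, then draws shared face, hair and tie parts, with lower hair on a coin flip.
; It returns the parts for a caller to apply, but its body type output reads a local this graph never assigns.
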(event EventBeginPlay
  (bind _hud_ref (Variables|Default|GetHUD_Ref))
  (bind _wbp_canteen (Variables|/Game/UI/WBP_HUD.WBP_HUD_C|GetWBP_Canteen _hud_ref))
  (Utilities|IsValid _wbp_canteen
    (:Is%20Valid
      (Default|KidSprite _wbp_canteen))))

(fn ConstructionScript
  (|CallParentFunction))

(fn GenerateLook
  (bind _eyebrowtypes (Variables|Looks|GeteyebrowTypes))
  (bind _eyetypes (Variables|Looks|GeteyeTypes))
  (bind _upperhairtypes (Variables|Looks|GetupperHairTypes))
  (bind _lowerhairtypes (Variables|Looks|GetlowerHairTypes))
  (bind _mouthtypes (Variables|Looks|GetmouthTypes))
  (bind _tietypes (Variables|Looks|GettieTypes))
  (bind _ba_clothings (Variables|Looks|GetbA_Clothings))
  (bind _bb_clothings (Variables|Looks|GetbB_Clothings))
  (bind _bc_clothings (Variables|Looks|GetbC_Clothings))
  (bind _bd_clothings (Variables|Looks|GetbD_Clothings))
  (bind _be_clothings (Variables|Looks|GetbE_Clothings))
  (bind _ba_blazer (Variables|Looks|GetbA_Blazer))
  (bind _bb_blazer (Variables|Looks|GetbB_Blazer))
  (bind _bc_blazer (Variables|Looks|GetbC_Blazer))
  (bind _bd_blazer (Variables|Looks|GetbD_Blazer))
  (bind _be_blazer (Variables|Looks|GetbE_Blazer))
  (bind _be_skintone (Variables|Looks|GetbE_SkinTone))
  (bind _bd_skintone (Variables|Looks|GetbD_SkinTone))
  (bind _bc_skintone (Variables|Looks|GetbC_SkinTone))
  (bind _bb_skintone (Variables|Looks|GetbB_SkinTone))
  (bind _ba_skintone (Variables|Looks|GetbA_SkinTone))
  (bind _output_get (LocalVariables|SetlocalBodyType (Math|Random|RandomIntegerinRange 0 (- (Utilities|Array|Length (Variables|Looks|GetbodyTypes)) 1))))
  (switch int _output_get
    (:0
      (LocalVariables|SetlocalClothingSelected (Utilities|Array|Get(acopy) _ba_clothings (Math|Random|RandomIntegerinRange 0 (- (Utilities|Array|Length _ba_clothings) 1))))
      (LocalVariables|SetlocalBlazerSelected (Utilities|Array|Get(acopy) _ba_blazer (Math|Random|RandomIntegerinRange 0 (- (Utilities|Array|Length _ba_blazer) 1))))
      (LocalVariables|SetlocalSkinToneSelected (Utilities|Array|Get(acopy) _ba_skintone (Math|Random|RandomIntegerinRange 0 (- (Utilities|Array|Length _ba_skintone) 1)))))
    (:1
      (LocalVariables|SetlocalClothingSelected (Utilities|Array|Get(acopy) _bb_clothings (Math|Random|RandomIntegerinRange 0 (- (Utilities|Array|Length _bb_clothings) 1))))
      (LocalVariables|SetlocalBlazerSelected (Utilities|Array|Get(acopy) _bb_blazer (Math|Random|RandomIntegerinRange 0 (- (Utilities|Array|Length _bb_blazer) 1))))
      (LocalVariables|SetlocalSkinToneSelected (Utilities|Array|Get(acopy) _bb_skintone (Math|Random|RandomIntegerinRange 0 (- (Utilities|Array|Length _bb_skintone) 1)))))
    (:2
      (LocalVariables|SetlocalClothingSelected (Utilities|Array|Get(acopy) _bc_clothings (Math|Random|RandomIntegerinRange 0 (- (Utilities|Array|Length _bc_clothings) 1))))
      (LocalVariables|SetlocalBlazerSelected (Utilities|Array|Get(acopy) _bc_blazer (Math|Random|RandomIntegerinRange 0 (- (Utilities|Array|Length _bc_blazer) 1))))
      (LocalVariables|SetlocalSkinToneSelected (Utilities|Array|Get(acopy) _bc_skintone (Math|Random|RandomIntegerinRange 0 (- (Utilities|Array|Length _bc_skintone) 1)))))
    (:3
      (LocalVariables|SetlocalClothingSelected (Utilities|Array|Get(acopy) _bd_clothings (Math|Random|RandomIntegerinRange 0 (- (Utilities|Array|Length _bd_clothings) 1))))
      (LocalVariables|SetlocalBlazerSelected (Utilities|Array|Get(acopy) _bd_blazer (Math|Random|RandomIntegerinRange 0 (- (Utilities|Array|Length _bd_blazer) 1))))
      (LocalVariables|SetlocalSkinToneSelected (Utilities|Array|Get(acopy) _bd_skintone (Math|Random|RandomIntegerinRange 0 (- (Utilities|Array|Length _bd_skintone) 1)))))
    (:4
      (LocalVariables|SetlocalClothingSelected (Utilities|Array|Get(acopy) _be_clothings (Math|Random|RandomIntegerinRange 0 (- (Utilities|Array|Length _be_clothings) 1))))
      (LocalVariables|SetlocalBlazerSelected (Utilities|Array|Get(acopy) _be_blazer (Math|Random|RandomIntegerinRange 0 (- (Utilities|Array|Length _be_blazer) 1))))
      (LocalVariables|SetlocalSkinToneSelected (Utilities|Array|Get(acopy) _be_skintone (Math|Random|RandomIntegerinRange 0 (- (Utilities|Array|Length _be_skintone) 1))))))
  (Utilities|FlowControl|Sequence
    (:then_0
      (LocalVariables|SetlocalEyeBrowSelected (Utilities|Array|Get(acopy) _eyebrowtypes (Math|Random|RandomIntegerinRange 0 (- (Utilities|Array|Length _eyebrowtypes) 1)))))
    (:then_1
      (LocalVariables|SetlocalEyeSelected (Utilities|Array|Get(acopy) _eyetypes (Math|Random|RandomIntegerinRange 0 (- (Utilities|Array|Length _eyetypes) 1))))
      (Utilities|FlowControl|Sequence
        (:then_0
          (LocalVariables|SetlocalUpperHairSelected (Utilities|Array|Get(acopy) _upperhairtypes (Math|Random|RandomIntegerinRange 0 (- (Utilities|Array|Length _upperhairtypes) 1)))))
        (:then_1
          (if (not (Math|Random|RandomBool))
            _
            (else
              (LocalVariables|SetlocalLowerHairSelected (Utilities|Array|Get(acopy) _lowerhairtypes (Math|Random|RandomIntegerinRange 0 (- (Utilities|Array|Length _lowerhairtypes) 1))))))
          (LocalVariables|SetlocalMouthSelected (Utilities|Array|Get(acopy) _mouthtypes (Math|Random|RandomIntegerinRange 0 (- (Utilities|Array|Length _mouthtypes) 1))))
          (LocalVariables|SetlocalTieSelected (Utilities|Array|Get(acopy) _tietypes (Math|Random|RandomIntegerinRange 0 (- (Utilities|Array|Length _tietypes) 1))))
          (return (LocalVariables|GetlocalBodyTypeSelected) (LocalVariables|GetlocalClothingSelected) (LocalVariables|GetlocalEyeSelected) (LocalVariables|GetlocalEyeBrowSelected) (LocalVariables|GetlocalUpperHairSelected) (LocalVariables|GetlocalLowerHairSelected) (LocalVariables|GetlocalMouthSelected) (LocalVariables|GetlocalTieSelected) (LocalVariables|GetlocalBlazerSelected) (LocalVariables|GetlocalSkinToneSelected)))))))