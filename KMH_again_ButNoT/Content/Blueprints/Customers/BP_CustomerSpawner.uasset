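; Customer spawner actor that starts the day's customer flow at BeginPlay.
; It rolls a random expected customer count and pushes it, with the served count, to the HUD.
; If no customer is waiting, it spawns a BPC_Customer with a random favourite food, the served count as its index and the HUD reference, then flags a customer as waiting.
; Only this first spawn happens here.
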(event EventBeginPlay
  (bind _listoffoods (Variables|Default|GetlistOfFoods))
  (bind _hud_ref (Variables|Default|GetHUD_Ref))
  ;[1 1 1] Generate Total Customers for the day
  (bind _output_get (Variables|Default|SetExpectedCustomers (Math|Random|RandomIntegerinRange 3 10)))
  (Development|PrintString (Utilities|String|ToString(Text) (Utilities|Text|FormatText "Expected Customer Count for the day is: {x}" _output_get)) false false)
  ;[1 1 1] Update the UI for the total count
  (Utilities|IsValid _hud_ref
    (:Is%20Valid
      (Default|UpdateCustomerCounter _hud_ref (Variables|Default|GetExpectedCustomers) (Variables|Default|GetServedCustomers))
      (if (not (Variables|Default|GetisCustomerWaiting?))
        ;[1 1 1] Get Favourite Food
        (Variables|Default|SetfavouriteFood (Utilities|Array|Get(acopy) _listoffoods (Math|Random|RandomIntegerinRange 0 (Utilities|Array|Length _listoffoods))))
        ;[1 1 1] Get Kid
        (bind _returnvalue (Game|SpawnActorfromClass "/Game/Blueprints/Customers/BPC_Customer.BPC_Customer_C" (Math|Transform|MakeTransform "0, 0, 0" "0, 0, 0" "1.000000,1.000000,1.000000") "Undefined" 0 (Variables|Default|GetServedCustomers) (Variables|Default|GetfavouriteFood) (Variables|Default|GetHUD_Ref) 0))
        (Variables|BP_CustomerSpawner_C|SetKidRef self _returnvalue)
        ;[1 1 1] Prevent Multiple Customers
        (Variables|Default|SetisCustomerWaiting? true)))
    (:Is%20Not%20Valid
      (Development|PrintString "invalid hud"))))

(fn ConstructionScript)